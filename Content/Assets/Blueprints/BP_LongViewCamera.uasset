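; BP_LongViewCamera is a one-shot trigger for a long-view camera, marked by a particle effect.
; When BP_Chromarion or BP_AcrylP first overlaps its Box, it sets LongViewActivated and plays the camera-switch sound.
; It then sets IsDeactivated to block retriggering and switches off the particle system.
; The graph only raises the flag and contains no camera view change itself.
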(event `self.Box.OnComponentBeginOverlap`
  (params (OverlappedComponent :type "PrimitiveComponent Object Reference") (OtherActor :type "Actor Object Reference") (OtherComp :type "PrimitiveComponent Object Reference") (OtherBodyIndex :type Integer) (bFromSweep :type Boolean) (SweepResult :type "HitResult Structure (by ref)"))
  (if (not (`self.IsDeactivated`))
    (cast `/Game/Characters/Chromarion/BP_Chromarion` OtherActor
      (:`then`
        (set `self.LongViewActivated` true)
        (`GameplayStatics.PlaySound2D` "/Game/Assets/Decors/Level_Mechanics/SFX/SwitchCamSoundEffect.SwitchCamSoundEffect" 1.0 1.0 0.0 null null))
      (:`CastFailed`
        (cast `/Game/Characters/Acryl/BP_AcrylP` OtherActor)
        (set `self.LongViewActivated` true)
        (`GameplayStatics.PlaySound2D` "/Game/Assets/Decors/Level_Mechanics/SFX/SwitchCamSoundEffect.SwitchCamSoundEffect" 1.0 1.0 0.0 null null)))
    (set `self.IsDeactivated` true)
    (`ActorComponent.Deactivate` (`self.ParticleSystem`))))

(fn `UserConstructionScript`)
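; BP_Cannon is a cannon actor that shows a lit fuse and fires cannonballs.
; On BeginPlay, if flagged as platform-mounted, it attaches to its linked platform and disables mesh physics simulation.
; BPPlaySFX activates the fuse effect, while BPShot triggers the explosion, stops the fuse and spawns a BP_CanonBall.
; The ball spawns at a fixed world-space offset from the explosion component, independent of cannon rotation.
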(event `self.ReceiveBeginPlay`
  (if (`self.bIsAttachedToPlatform`)
    (`self.K2_AttachToActor` self (`self.Linkedplatform`) "None" "KeepWorld" "KeepWorld" "KeepWorld" true)
    (`PrimitiveComponent.SetSimulatePhysics` (`self.StaticMesh`) false)))

(event `self.BPPlaySFX`
  (`ActorComponent.Activate` (`self.LitFuse`) false))

(event `self.BPShot`
  (`ActorComponent.Activate` (`self.Explosion`) false)
  (`ActorComponent.Deactivate` (`self.LitFuse`))
  (`|SpawnActorFromClass` "/Game/Assets/Blueprints/BP_CanonBall.BP_CanonBall_C" (`KismetMathLibrary.Conv_VectorToTransform` (+ (`SceneComponent.GetSocketLocation` (`self.Explosion`) "None") (-100.0 20.0 40.0))) "Undefined" "MultiplyWithRoot" null null))

(fn `UserConstructionScript`)
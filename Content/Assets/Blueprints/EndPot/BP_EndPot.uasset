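; End-of-level pot actor that completes the level once two ColorLeak characters overlap it, and also opens the start-level widget on BeginPlay.
; On completion it records time and progress with the game mode and instance, plays victory sound and animations, and swaps LevelObjects materials from normal to grey via path-name replacement.
; A timeline returns the camera to its starting position, then the game pauses and shows the level-complete or last-level widget.
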(event `self.ReceiveActorBeginOverlap`
  (params (OtherActor :type "Actor Object Reference"))
  (cast `ColorLeakCharacter` OtherActor)
  (bind _output_get (set `self.NbPlayer` (+ (`self.NbPlayer`) 1)))
  (if (== _output_get 2)
    (`self.AllPlayersIn`)))

(event `self.ReceiveActorEndOverlap`
  (params (OtherActor :type "Actor Object Reference"))
  (cast `ColorLeakCharacter` OtherActor)
  (set `self.NbPlayer` (+ (`self.NbPlayer`) -1)))

(event `AllPlayersIn`
  (bind _returnvalue (`GameplayStatics.GetPlayerController` 0))
  (bind _returnvalue_2 (`GameplayStatics.GetPlayerController` 0))
  (bind _ascolor_leak_game_mode (cast `ColorLeakGameMode` (`GameplayStatics.GetGameMode`)))
  (`ColorLeakGameMode.AddIGT` _ascolor_leak_game_mode)
  (bind _ascolor_leak_game_instance (cast `ColorLeakGameInstance` (`GameplayStatics.GetGameInstance`)))
  (`ColorLeakGameInstance.FinishLevel` _ascolor_leak_game_instance (`self.Level`))
  (if (`self.LastLevel`)
    (`ColorLeakGameInstance.SetRealEndTime` _ascolor_leak_game_instance))
  (`GameplayStatics.PlaySound2D` "/Game/Characters/Acryl/Sounds/victory_sound.victory_sound" 1.0 1.0 0.0 null null)
  (bind _outactors (`GameplayStatics.GetAllActorsOfClassWithTag` "/Script/Engine.Actor" "LevelObjects"))
  (for _array_element _outactors
    (for _array_element_2 (`self.K2_GetComponentsByClass` _array_element "/Script/Engine.StaticMeshComponent")
      (for _index (range (`PrimitiveComponent.GetNumMaterials` _array_element_2))
        (`PrimitiveComponent.SetMaterial` _array_element_2 _index (`PrimitiveComponent.GetMaterialByName` (`self.StaticMesh`) (`KismetStringLibrary.Conv_StringToName` (`KismetStringLibrary.Replace` (`KismetSystemLibrary.GetPathName` (`PrimitiveComponent.GetMaterial` _array_element_2 _index)) "Normal_Color" "Grey_Color"))))
        (bind _returnvalue_3 (`GameplayStatics.GetActorOfClass` "/Script/ColorLeak.Acryl"))
        (`self.DisableInput` _returnvalue_3 (`GameplayStatics.GetPlayerController` 0))
        (`self.K2_SetActorRotation` _returnvalue_3 (struct :`Yaw` 180.0) false)
        (`KismetSystemLibrary.Delay` 0.2)
        (`SkeletalMeshComponent.PlayAnimation` (`Character.Mesh` _returnvalue_3) "/Game/Characters/Acryl/Animations/Anim_Victory.Anim_Victory" false)
        (bind _returnvalue_4 (`GameplayStatics.GetActorOfClass` "/Script/ColorLeak.Chromarion"))
        (`self.DisableInput` _returnvalue_4 (`GameplayStatics.GetPlayerController` 1))
        (`self.K2_SetActorRotation` _returnvalue_4 (struct :`Yaw` 180.0) false)
        (`SkeletalMeshComponent.PlayAnimation` (`Character.Mesh` _returnvalue_4) "/Game/Characters/Chromarion/Animations/Yes.Yes" false)
        (set `self.CameraEnd` (`self.K2_GetActorLocation` (`self.Camera`)))
        (`KismetSystemLibrary.Delay` 2.0)
        (bind (_direction _cameratravel) (`Timeline|Chronologie`)
          (:`Update`
            (`self.K2_SetActorLocation` (`self.Camera`) (`KismetMathLibrary.VLerp` (`self.CameraEnd`) (`self.CameraStart`) _cameratravel) false false))
          (:`Finished`
            (`self.K2_SetActorLocation` (`self.Camera`) (`self.CameraStart`) false false)
            (`GameplayStatics.SetGamePaused` true)
            (if (`self.LastLevel`)
              (bind _returnvalue_5 (`|CreateWidget` "/Game/UI/Levels/WB_LastLevelComplete.WB_LastLevelComplete_C" _returnvalue_2 (`self.Next Level`) (`self.Level`)))
              (`UserWidget.AddToViewport` _returnvalue_5 0)
              (`WidgetBlueprintLibrary.SetInputMode_UIOnlyEx` _returnvalue_2 _returnvalue_5)
              (`KismetSystemLibrary.Delay` 0.2)
              (`Widget.SetKeyboardFocus` (`/Game/UI/Levels/WB_LastLevelComplete.Button_MainMenu` _returnvalue_5))
              (else
                (bind _returnvalue_6 (`|CreateWidget` "/Game/UI/Levels/WB_LevelComplete.WB_LevelComplete_C" _returnvalue (`self.Next Level`) (`self.Level`)))
                (`UserWidget.AddToViewport` _returnvalue_6 0)
                (`WidgetBlueprintLibrary.SetInputMode_UIOnlyEx` _returnvalue _returnvalue_6)
                (`KismetSystemLibrary.Delay` 0.2)
                (`Widget.SetKeyboardFocus` (`/Game/UI/Levels/WB_LevelComplete.Button_NextLevel` _returnvalue_6))))
            (`self.EnableInput` _returnvalue_3 (`GameplayStatics.GetPlayerController` 0))
            (`self.EnableInput` _returnvalue_4 (`GameplayStatics.GetPlayerController` 1))))))))

(event `self.ReceiveBeginPlay`
  (bind _returnvalue (`|CreateWidget` "/Game/UI/Levels/WB_StartLevel.WB_StartLevel_C" null (`self.Level Name`)))
  (`UserWidget.AddToViewport` _returnvalue 50)
  (`GameplayStatics.SetGamePaused` true)
  (`WidgetBlueprintLibrary.SetInputMode_GameAndUIEx` (`GameplayStatics.GetPlayerController` 0) _returnvalue)
  (bind _returnvalue_2 (`GameplayStatics.GetActorOfClass` "/Script/Engine.CameraActor"))
  (bind _output_get (set `self.Camera` _returnvalue_2))
  (set `self.CameraStart` (`self.K2_GetActorLocation` _output_get)))

(fn `UserConstructionScript`)
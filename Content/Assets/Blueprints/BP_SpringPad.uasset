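; BP_SpringPad is a bounce pad that launches the BP_AcrylP and BP_Chromarion characters upward when they overlap its box collision.
; It overwrites the character's vertical velocity with a per-character jump value multiplied by a gravity scale, keeping horizontal velocity intact.
; Both cases then share a one-shot bounce animation on the skeletal mesh and a 2D spring sound, while other actors are ignored.
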(event `self.BoxCollision.OnComponentBeginOverlap`
  (params (OverlappedComponent :type "PrimitiveComponent Object Reference") (OtherActor :type "Actor Object Reference") (OtherComp :type "PrimitiveComponent Object Reference") (OtherBodyIndex :type Integer) (bFromSweep :type Boolean) (SweepResult :type "HitResult Structure (by ref)"))
  (bind _asbp_acryl_p (cast `/Game/Characters/Acryl/BP_AcrylP` OtherActor)
    (:`then`
      (bind (_returnvalue_x _returnvalue_y) (`KismetMathLibrary.BreakVector` (`self.GetVelocity` _asbp_acryl_p)))
      (set `MovementComponent.Velocity` (`KismetMathLibrary.MakeVector` _returnvalue_x _returnvalue_y (* (`self.AcrylJumpValue`) (`self.GravityScale`))) (`Character.CharacterMovement` _asbp_acryl_p)))
    (:`CastFailed`
      (bind _asbp_chromarion (cast `/Game/Characters/Chromarion/BP_Chromarion` OtherActor))
      (bind (_returnvalue_x_2 _returnvalue_y_2) (`KismetMathLibrary.BreakVector` (`self.GetVelocity` _asbp_chromarion)))
      (set `MovementComponent.Velocity` (`KismetMathLibrary.MakeVector` _returnvalue_x_2 _returnvalue_y_2 (* (`self.ChromaionJumpValue`) (`self.GravityScale`))) (`Character.CharacterMovement` _asbp_chromarion))))
  (`SkeletalMeshComponent.PlayAnimation` (`self.SkeletalMesh`) "/Game/Assets/Decors/Level_Mechanics/Bouncer_Anim_Bouncer_Bounce.Bouncer_Anim_Bouncer_Bounce" false)
  (`GameplayStatics.PlaySound2D` "/Game/Assets/Decors/Level_Mechanics/SFX/Spring_Bounces.Spring_Bounces" 1.0 1.0 0.0 null null))

(fn `UserConstructionScript`)
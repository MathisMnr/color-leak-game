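; Cannonball projectile that explodes on contact, killing player characters and breaking destructible blocks.
; On BeginPlay it disables gravity on the Bomb, launches and spins it with impulses, then explodes after a short fuse.
; Box overlaps spawn the explosion, destroy the ball, and call DeathCharacter on BP_AcrylP or BP_Chromarion, or destroy a BP_DestructibleBlock.
; Timeout and block-hit sounds play at world origin; only character hits place the sound at the impact.
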(event `self.ReceiveBeginPlay`
  (bind _bomb (`self.Bomb`))
  (`PrimitiveComponent.SetEnableGravity` _bomb false)
  (`PrimitiveComponent.AddImpulse` _bomb (* (`SceneComponent.GetForwardVector` _bomb) (0.0 -1000.0 0.85)) "None" true)
  (`PrimitiveComponent.AddAngularImpulseInDegrees` (`self.Bomb`) (30.0 20.0 15.0) "None" true)
  (`KismetSystemLibrary.Delay` 3.0)
  (`GameplayStatics.SpawnEmitterAtLocation` "/Game/StarterContent/Particles/P_Explosion.P_Explosion" (`SceneComponent.GetSocketLocation` (`self.Bomb`) "None") (struct) (1.5 1.5 1.5))
  (`self.K2_DestroyActor` self)
  (`GameplayStatics.PlaySoundAtLocation` "/Game/Assets/Decors/Level_Mechanics/SFX/Bomb_Explosion_Sound_Effect.Bomb_Explosion_Sound_Effect" (0.0 0.0 0.0) (struct) 1.0 1.0 0.0 null null null null))

(event `self.Box.OnComponentBeginOverlap`
  (params (OverlappedComponent :type "PrimitiveComponent Object Reference") (OtherActor :type "Actor Object Reference") (OtherComp :type "PrimitiveComponent Object Reference") (OtherBodyIndex :type Integer) (bFromSweep :type Boolean) (SweepResult :type "HitResult Structure (by ref)"))
  (bind _ascolor_leak_character (cast `ColorLeakCharacter` OtherActor)
    (:`then`
      (bind _returnvalue (`CharacterMovementComponent.GetLastUpdateLocation` (`Character.CharacterMovement` _ascolor_leak_character)))
      (`GameplayStatics.SpawnEmitterAtLocation` "/Game/StarterContent/Particles/P_Explosion.P_Explosion" _returnvalue (struct) (1.5 1.5 1.5))
      (`self.K2_DestroyActor` self)
      (`GameplayStatics.PlaySoundAtLocation` "/Game/Assets/Decors/Level_Mechanics/SFX/Bomb_Explosion_Sound_Effect.Bomb_Explosion_Sound_Effect" _returnvalue (struct) 1.0 1.0 0.0 null null null null)
      (bind _asbp_acryl_p (cast `/Game/Characters/Acryl/BP_AcrylP` _ascolor_leak_character)
        (:`then`
          (`Acryl.DeathCharacter` _asbp_acryl_p))
        (:`CastFailed`
          (bind _asbp_chromarion (cast `/Game/Characters/Chromarion/BP_Chromarion` _ascolor_leak_character))
          (`Chromarion.DeathCharacter` _asbp_chromarion))))
    (:`CastFailed`
      (bind _asbp_destructible_block (cast `/Game/Assets/Blueprints/BP_DestructibleBlock` OtherActor))
      (`GameplayStatics.SpawnEmitterAtLocation` "/Game/StarterContent/Particles/P_Explosion.P_Explosion" (`self.K2_GetActorLocation` _asbp_destructible_block) (struct) (1.5 1.5 1.5))
      (`self.K2_DestroyActor` self)
      (`GameplayStatics.PlaySoundAtLocation` "/Game/Assets/Decors/Level_Mechanics/SFX/Bomb_Explosion_Sound_Effect.Bomb_Explosion_Sound_Effect" (0.0 0.0 0.0) (struct) 1.0 1.0 0.0 null null null null)
      (`self.K2_DestroyActor` _asbp_destructible_block))))

(fn `UserConstructionScript`)
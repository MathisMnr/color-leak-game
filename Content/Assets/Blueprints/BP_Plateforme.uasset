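; BP_Plateforme is a platform that lowers while a BP_AcrylP or Chromarion actor stands on it.
; Overlap events raise and lower an OnPlateform counter of those occupants.
; Each qualifying entry plays a timeline that drives the static mesh's relative Z location, and the timeline reverses only when the count returns to zero, so the platform stays down while anyone remains.
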(event `self.ReceiveActorBeginOverlap`
  (params (OtherActor :type "Actor Object Reference"))
  (cast `/Game/Characters/Acryl/BP_AcrylP` OtherActor
    (:`then`
      _)
    (:`CastFailed`
      (cast `Chromarion` OtherActor)))
  (set `self.OnPlateform` (+ (`self.OnPlateform`) 1))
  (bind (_direction _lowering) (`Timeline|TL_Lowering_Plateform` :!label _label)
    (:`Update`
      (`SceneComponent.K2_SetRelativeLocation` (`self.StaticMesh`) (`KismetMathLibrary.MakeVector` 0.0 0.0 _lowering) false false))))

(event `self.ReceiveActorEndOverlap`
  (params (OtherActor :type "Actor Object Reference"))
  (cast `/Game/Characters/Acryl/BP_AcrylP` OtherActor
    (:`then`
      _)
    (:`CastFailed`
      (cast `Chromarion` OtherActor)))
  (bind _output_get (set `self.OnPlateform` (+ (`self.OnPlateform`) -1)))
  (if (== _output_get 0)
    (goto _label :!via `Reverse`)))

(fn `UserConstructionScript`)
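; Lobby game mode in the test levels folder that removes an extra local player when the level starts.
; On BeginPlay, if more than one player exists, it destroys the pawn and controller at player index 1.
; It then switches player 0's view target to that player's own pawn, provided the pawn is a Character.
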(event `self.ReceiveBeginPlay`
  (bind _returnvalue (`GameplayStatics.GetPlayerController` 1))
  (bind _returnvalue_2 (`GameplayStatics.GetPlayerController` 0))
  (bind _returnvalue_3 (`self.GetNumPlayers`))
  (if (> _returnvalue_3 1)
    (`self.K2_DestroyActor` (`Controller.K2_GetPawn` _returnvalue))
    (`self.K2_DestroyActor` _returnvalue)
    (bind _ascharacter (cast `Character` (`Controller.K2_GetPawn` _returnvalue_2)))
    (`PlayerController.SetViewTargetWithBlend` _returnvalue_2 _ascharacter 0.0 "VTBlend_Linear" 0.0 false)))

(fn `UserConstructionScript`)